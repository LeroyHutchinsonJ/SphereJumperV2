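; Collectible gem actor that adds score to the player on overlap and then destroys itself.
; The overlap handler casts the other actor to Player and passes ScoreToGive to its AddScore.
; Each Tick spins the mesh in yaw by RotateSpeed and bobs it with a sine of real time.
; The spin scales with delta time, while the bob adds a per-frame offset, so its height depends on frame rate.
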(event `self.ReceiveActorBeginOverlap`
  (params (OtherActor :type "Actor Object Reference"))
  ;[1 1 1] Player Collecting
  (bind _asplayer (cast `/Game/Blueprints/Player` OtherActor))
  (`/Game/Blueprints/Player.Add Score` _asplayer (`self.ScoreToGive`))
  (`self.K2_DestroyActor`))

(event `self.ReceiveTick`
  (params (DeltaSeconds :type "Float (single-precision)"))
  ;[1 1 1] Gem Movement
  (`SceneComponent.K2_AddWorldRotation` (`self.StaticMesh`) (`KismetMathLibrary.MakeRotator` 0.0 0.0 (* DeltaSeconds (`self.RotateSpeed`))) false false)
  (`SceneComponent.K2_AddWorldOffset` (`self.StaticMesh`) (`KismetMathLibrary.MakeVector` 0.0 0.0 (/ (`KismetMathLibrary.Sin` (* (`GameplayStatics.GetRealTimeSeconds`) 2.0)) 2.0)) false false))

(fn `UserConstructionScript`)